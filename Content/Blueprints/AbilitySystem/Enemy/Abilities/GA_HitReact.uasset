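; Enemy hit react gameplay ability that applies GE_HitReact to its owner and plays a hit reaction montage.
; The montage comes from the avatar through CombatInterface.
; When it completes, is interrupted or is cancelled, the ability removes the effect by its stored handle and ends.
; A debug line drawn from the avatar's location visualizes the reported hit direction.
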(event `self.K2_ActivateAbility`
  (bind _returnvalue (`self.GetAvatarActorFromActorInfo`))
  (bind _returnvalue_2 (message `CombatInterface.GetHitDirection` _returnvalue))
  (`self.DrawDebugHitDirectionLine` (`Actor.K2_GetActorLocation` _returnvalue) _returnvalue_2)
  (bind _returnvalue_3 (`self.BP_ApplyGameplayEffectToOwner` "/Game/Blueprints/AbilitySystem/Enemy/Effects/GE_HitReact.GE_HitReact_C"))
  (set `self.Active GE Hit React` _returnvalue_3)
  (bind _ascombat_interface (cast `CombatInterface` (`self.GetAvatarActorFromActorInfo`)))
  (bind _returnvalue_4 (`CombatInterface.GetHitReactMontage` _ascombat_interface))
  (`AbilityTask_PlayMontageAndWait.CreatePlayMontageAndWaitProxy` "None" _returnvalue_4
    (:`OnCompleted`
      _)
    (:`OnInterrupted`
      _)
    (:`OnCancelled`
      _))
  (`self.BP_RemoveGameplayEffectFromOwnerWithHandle` (`self.Active GE Hit React`))
  (`self.K2_EndAbility`))

(fn `DrawDebugHitDirectionLine`
  (params (LineStart :type "Vector Structure") (Direction :type "Vector Structure"))
  (`KismetSystemLibrary.DrawDebugLine` LineStart (- LineStart (* (`KismetMathLibrary.Normal` Direction) 100)) (struct :`R` 0.932292 :`G` 0.324354 :`A` 1.0) 5.0 1.0))