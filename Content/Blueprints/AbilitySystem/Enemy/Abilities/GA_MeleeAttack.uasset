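; Enemy melee attack ability, instanced per actor, that turns the avatar toward its combat target and plays a random tagged attack montage.
; The montage's gameplay event triggers a small sphere query at the tagged combat socket, applying class-default damage to live non-friends.
; If anything is hit, a MeleeImpact gameplay cue carries the montage tag and location in place of direct sound playback.
; The ability ends after the strike or when the montage finishes or is interrupted.
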(event `self.K2_ActivateAbility`
  (bind _returnvalue (`self.GetAvatarActorFromActorInfo`))
  (bind _returnvalue_2 (`self.GetAvatarActorFromActorInfo`))
  (bind (_taggedmontage_montage _taggedmontage_montagetag) (break `TaggedMontage` (`self.TaggedMontage`)))
  ;[1 1 1] Instanced Per Actor
  (set `self.HasHitTarget` false)
  (`|ExecutionSequence`
    (:`then_0`
      (bind _returnvalue_3 (message `EnemyInterface.GetCombatTarget` _returnvalue_2))
      (message `CombatInterface.UpdateFacingTarget` _returnvalue_2 (`Actor.K2_GetActorLocation` _returnvalue_3)))
    (:`then_1`
      (bind _returnvalue_4 (message `CombatInterface.GetAttackMontages` (`self.GetAvatarActorFromActorInfo`)))
      (bind _output_get (set `self.TaggedMontage` (`self.GetRandomTaggedMontageFromArray` _returnvalue_4)))
      (bind (_montage _montagetag _sockettag) (break `TaggedMontage` _output_get))
      (`AbilityTask_PlayMontageAndWait.CreatePlayMontageAndWaitProxy` "None" _montage 1.0 "None" false
        (:`then`
          (`AbilityTask_WaitGameplayEvent.WaitGameplayEvent` _montagetag null
            (:`EventReceived`
              ;[1 1 1] Socket Tag
              (bind _returnvalue_5 (message `CombatInterface.GetCombatSocketLocation` _returnvalue _sockettag))
              (bind _output_get_2 (set `self.CombatSocketLocation` _returnvalue_5))
              (bind _outoverlappingactors (`AuraAbilitySystemLibrary.GetLivePlayersWithinRadius` self (`|MakeArray` _returnvalue) 45.0 _output_get_2))
              (for _array_element _outoverlappingactors
                (if (`AuraAbilitySystemLibrary.IsNotFriend` _array_element (`self.GetAvatarActorFromActorInfo`))
                  (`AuraAbilitySystemLibrary.ApplyDamageEffect` (`self.MakeDamageEffectParamsFromClassDefaults` _array_element))
                  ;[0.08979 0.1584 0.1667] Hit Particle On Server
                  (set `self.HasHitTarget` true)
                  (bind _returnvalue_6 (message `CombatInterface.GetBloodEffect` _array_element))))
              (`|ExecutionSequence`
                (:`then_0`
                  ;[0.08979 0.1584 0.1667] Sound On Server
                  (if (`self.HasHitTarget`)
                    ;[0.5387 0.9502 1] Use Cue Instead
                    (bind _returnvalue_7 (message `EnemyInterface.GetCombatTarget` (`self.GetAvatarActorFromActorInfo`)))
                    (`self.K2_ExecuteGameplayCueWithParams` (struct :`TagName` "GameplayCue.MeleeImpact") (`AbilitySystemBlueprintLibrary.MakeGameplayCueParameters` 0.0 0.0 (struct) (struct) (struct) (`BlueprintGameplayTagLibrary.MakeGameplayTagContainerFromTag` _taggedmontage_montagetag) (struct) (`self.CombatSocketLocation`) (0.0 0.0 0.0) null (`self.GetAvatarActorFromActorInfo`) _returnvalue_7))))
                (:`then_1`
                  (`self.K2_EndAbility`))))))
        (:`OnCompleted`
          (`self.K2_EndAbility` :!label _label))
        (:`OnInterrupted`
          (goto _label))
        (:`OnCancelled`
          (goto _label))))))

(event `self.K2_OnEndAbility`
  (params (bWasCancelled :type Boolean)))