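; Enemy gameplay ability for a ranged attack that fires a projectile at the avatar's combat target.
; On activation it gets the target through interface-style messages, sets it as the motion-warping facing target and caches its location.
; It plays a random tagged montage from the character's attack montages and waits for that montage's gameplay event.
; The event spawns the projectile from the tagged socket with a pitch override, then ends the ability.
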(event `self.K2_ActivateAbility`
  (bind _returnvalue (`self.GetAvatarActorFromActorInfo`))
  (`|ExecutionSequence`
    (:`then_0`
      ;[1 1 1] From Behavior Tree
      (bind _returnvalue_2 (message `EnemyInterface.GetCombatTarget` _returnvalue))
      (bind _returnvalue_3 (`Actor.K2_GetActorLocation` _returnvalue_2))
      ;[1 1 1] Motion Warping
      (message `CombatInterface.UpdateFacingTarget` _returnvalue _returnvalue_3)
      ;[1 1 1] Target Location
      (set `self.ProjectileTargetLocation` _returnvalue_3))
    (:`then_1`
      ;[1 1 1] From Character Blueprint
      (bind _returnvalue_4 (message `CombatInterface.GetAttackMontages` (`self.GetAvatarActorFromActorInfo`)))
      (bind _output_get (set `self.TaggedMontage` (`self.GetRandomTaggedMontageFromArray` _returnvalue_4)))
      (bind (_montage _montagetag _sockettag) (break `TaggedMontage` _output_get))
      (`AbilityTask_PlayMontageAndWait.CreatePlayMontageAndWaitProxy` "None" _montage 1.0 "None" false
        (:`then`
          (`AbilityTask_WaitGameplayEvent.WaitGameplayEvent` _montagetag null true
            (:`EventReceived`
              (`self.SpawnProjectile` (`self.ProjectileTargetLocation`) _sockettag true 25.0)
              (`self.K2_EndAbility`))))
        (:`OnCompleted`
          (`self.K2_EndAbility` :!label _label))
        (:`OnInterrupted`
          (goto _label))
        (:`OnCancelled`
          (goto _label))))))