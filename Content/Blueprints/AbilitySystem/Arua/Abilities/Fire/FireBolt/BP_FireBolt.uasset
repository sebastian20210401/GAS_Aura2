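; Fire Bolt projectile Blueprint for Arua's fire ability, with a Sphere collision component and a ProjectileMovement component.
; Its only live logic waits briefly after BeginPlay, then enables query-only collision on the Sphere.
; Disconnected leftover nodes would adjust or clear homing and draw a debug sphere, but never run.
; The graph itself contains no hit or damage handling.
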(event `self.ReceiveBeginPlay`
  (`KismetSystemLibrary.Delay` 0.05)
  (`PrimitiveComponent.SetCollisionEnabled` (`self.Sphere`) "QueryOnly"))

(fn `UserConstructionScript`)