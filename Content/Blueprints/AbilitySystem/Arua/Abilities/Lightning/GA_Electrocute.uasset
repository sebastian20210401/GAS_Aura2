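; Electrocute lightning gameplay ability that plays a looping cast while input is held; no damage or beam logic is present yet.
; For a CombatInterface avatar, it stores mouse target and owner data, hides the cursor, faces the target and fires the ShockBurst cue.
; An intro montage chains into a self-restarting loop montage, while input release restores the cursor and ends the ability.
; Movement disable and restore nodes exist but are disconnected.
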(event `self.K2_ActivateAbility`
  (if (`KismetSystemLibrary.DoesImplementInterface` (`self.GetAvatarActorFromActorInfo`) "/Script/Aura.CombatInterface")
    ;[1 1 1] Store Mouse Data
    (bind (_asynctaskproxy _datahandle) (`TargetDataUnderMouse.CreateTargetDataUnderMouse`)
      (:`ValidData`
        (`self.StoreMouseDataInfo` (`AbilitySystemBlueprintLibrary.GetHitResultFromTargetData` _datahandle))
        (`self.StoreOwnerVariables`)
        (`|ExecutionSequence`
          (:`then_0`
            (set `PlayerController.bShowMouseCursor` false (`self.OwnerPlayerController`))
            (message `CombatInterface.UpdateFacingTarget` (`self.GetAvatarActorFromActorInfo`) (`self.MouseHitLocation`))
            (`self.K2_ExecuteGameplayCue` (struct :`TagName` "GameplayCue.ShockBurst"))
            (`AbilityTask_PlayMontageAndWait.CreatePlayMontageAndWaitProxy` "None" (`self.Montage_Electrocute`) 1.0 "None" false
              (:`OnBlendOut`
                (`AbilityTask_PlayMontageAndWait.CreatePlayMontageAndWaitProxy` "None" (`self.Montage_Electrocute_Loop`) :!label _label
                  (:`OnBlendOut`
                    (goto _label))))))
          (:`then_1`
            (`AbilityTask_WaitInputRelease.WaitInputRelease` false
              (:`OnRelease`
                (set `PlayerController.bShowMouseCursor` true (`self.OwnerPlayerController`))
                (`self.K2_EndAbility`)))))))
    (else
      (`self.K2_EndAbility`))))