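; GA_ListenForEvent is a passive gameplay ability that turns attribute gameplay events into gameplay effects on its owner.
; On activation it waits for events under the Attributes tag, including child tags, and never ends itself.
; Each event builds a spec from EventBasedEffectClass, sets a SetByCaller magnitude keyed by the event's tag from its magnitude, and applies it to self.
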(event `self.K2_ActivateAbility`
  (bind _returnvalue (`self.GetAbilitySystemComponentFromActorInfo`))
  (`KismetSystemLibrary.PrintString` "Listening for Events")
  ;[1 1 1] No On EndAbility
  (bind (_asynctaskproxy _payload) (`AbilityTask_WaitGameplayEvent.WaitGameplayEvent` (struct :`TagName` "Attributes") null false false)
    (:`EventReceived`
      (bind (_eventtag _instigator _target _optionalobject _optionalobject2 _contexthandle _instigatortags _targettags _eventmagnitude) (break `GameplayEventData` _payload))
      (bind _returnvalue_2 (`AbilitySystemBlueprintLibrary.AssignTagSetByCallerMagnitude` (`AbilitySystemComponent.MakeOutgoingSpec` _returnvalue (`self.EventBasedEffectClass`) 0.0 (`AbilitySystemComponent.MakeEffectContext` _returnvalue)) _eventtag _eventmagnitude))
      (`AbilitySystemComponent.BP_ApplyGameplayEffectSpecToSelf` (`self.GetAbilitySystemComponentFromActorInfo`) _returnvalue_2))))