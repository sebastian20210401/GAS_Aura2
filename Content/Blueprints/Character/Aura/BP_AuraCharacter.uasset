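; Player character Blueprint for Aura, handling facing, camera-obstruction fading and some debug test hooks.
; UpdateFacingTarget feeds a Motion Warping target, while Z and X test a cast montage with and without it.
; FadeBox overlaps send fade messages to BI_Fade actors.
; A cooldown listener and timer track TimeRemaining, which E shortens by reapplying the FireBolt cooldown effect with a SetByCaller duration.
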(event `CombatInterface.UpdateFacingTarget`
  (params (Target :type "Vector Structure (by ref)"))
  (`MotionWarpingComponent.AddOrUpdateWarpTargetFromLocation` (`self.MotionWarping`) "FacingTarget" Target))

(event `Key|E`
  (params (Key :type "Key Structure"))
  ;[0.618 0.9299 1] Cooldown
  (:`Pressed`
    (`self.Server_ResetFireBoltCooldown` (`KismetMathLibrary.FMax` (- (`self.TimeRemaining`) 2.0) 0.1))))

(event `Server_ResetFireBoltCooldown`
  (params (Magnitude :type "Float (single-precision)" :default 2.0))
  (bind _returnvalue (`AbilitySystemBlueprintLibrary.GetAbilitySystemComponent` self))
  ;[0.618 0.9299 1] Cooldown
  (`AbilitySystemComponent.RemoveActiveEffectsWithTags` (`AbilitySystemBlueprintLibrary.GetAbilitySystemComponent` self) (struct :`GameplayTags` (struct :`(TagName` "Cooldown.Fire.FireBolt"))))
  (bind _returnvalue_2 (`AbilitySystemBlueprintLibrary.AssignTagSetByCallerMagnitude` (`AbilitySystemComponent.MakeOutgoingSpec` :`self` _returnvalue :`GameplayEffectClass` "/Game/Blueprints/AbilitySystem/Arua/Abilities/Fire/FireBolt/GE_DynamicCooldown_FireBolt.GE_DynamicCooldown_FireBolt_C") (struct :`TagName` "Tests.GenericTag") Magnitude))
  (`AbilitySystemComponent.BP_ApplyGameplayEffectSpecToSelf` _returnvalue _returnvalue_2))

(event `ANS_Test`
  ;[1 1 1] Motion Wrap
  (bind _ans_testactor (`self.ANS_TestActor`)
    (:`then`
      (`MotionWarpingComponent.AddOrUpdateWarpTargetFromLocation` (`self.MotionWarping`) "FacingTarget" (`self.K2_GetActorLocation` _ans_testactor)))
    (:`else`)))

(event `Key|F`
  (params (Key :type "Key Structure"))
  ;[0.618 0.9299 1] Cooldown
)

(event `self.ReceiveBeginPlay`
  ;[0.618 0.9299 1] Cooldown
  (bind (_asynctaskproxy _timeremaining) (`WaitCooldownChange.WaitForCooldownChange` (`AbilitySystemBlueprintLibrary.GetAbilitySystemComponent` self) (`self.CooldownTag`))
    (:`CooldownStart`
      (bind _output_get (set `self.TimeRemaining` _timeremaining))
      (`KismetSystemLibrary.K2_ClearAndInvalidateTimerHandle` (`self.CooldownTimerHandle`))
      (bind _returnvalue (`KismetSystemLibrary.K2_SetTimerDelegate` (delegate `UpdateTimer`) (`self.TimerFreq`) true))
      (set `self.CooldownTimerHandle` _returnvalue))))

(event `Key|Z`
  (params (Key :type "Key Structure"))
  ;[1 1 1] Motion Wrap
  (:`Pressed`
    (bind _ans_testactor (`self.ANS_TestActor`)
      (:`then`
        (`MotionWarpingComponent.AddOrUpdateWarpTargetFromLocation` (`self.MotionWarping`) "FacingTarget" (`self.K2_GetActorLocation` _ans_testactor))
        (`|PlayMontage` (`self.Mesh`) "/Game/Assets/Characters/Aura/Animations/Abilities/AM_Cast_ArcaneShards_Test.AM_Cast_ArcaneShards_Test"))
      (:`else`))))

(event `UpdateTimer`
  ;[0.618 0.9299 1] Cooldown
  (set `self.TimeRemaining` (- (`self.TimeRemaining`) (`self.TimerFreq`))))

(event `Key|X`
  (params (Key :type "Key Structure"))
  ;[1 1 1] Motion Wrap
  (:`Pressed`
    (`MotionWarpingComponent.RemoveWarpTarget` (`self.MotionWarping`) "FacingTarget")
    (`|PlayMontage` (`self.Mesh`) "/Game/Assets/Characters/Aura/Animations/Abilities/AM_Cast_ArcaneShards_Test.AM_Cast_ArcaneShards_Test")))

(event `self.FadeBox.OnComponentBeginOverlap`
  (params (OverlappedComponent :type "PrimitiveComponent Object Reference") (OtherActor :type "Actor Object Reference") (OtherComp :type "PrimitiveComponent Object Reference") (OtherBodyIndex :type Integer) (bFromSweep :type Boolean) (SweepResult :type "HitResult Structure (by ref)"))
  (if (`KismetSystemLibrary.DoesImplementInterface` OtherActor "/Game/Blueprints/Actor/FadeActor/BI_Fade.BI_Fade_C")
    (message `/Game/Blueprints/Actor/FadeActor/BI_Fade.FadeOut` OtherActor)))

(event `self.FadeBox.OnComponentEndOverlap`
  (params (OverlappedComponent :type "PrimitiveComponent Object Reference") (OtherActor :type "Actor Object Reference") (OtherComp :type "PrimitiveComponent Object Reference") (OtherBodyIndex :type Integer))
  (if (`KismetSystemLibrary.DoesImplementInterface` OtherActor "/Game/Blueprints/Actor/FadeActor/BI_Fade.BI_Fade_C")
    (message `/Game/Blueprints/Actor/FadeActor/BI_Fade.FadeIn` OtherActor)))

(fn `UserConstructionScript`)